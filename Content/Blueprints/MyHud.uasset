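; HUD that draws a drag selection box on screen and gathers the BaseVehicle actors inside it.
; Start and update events store the corner coordinates, and DrawHUD draws four lines and queries the rectangle each frame once the drag diagonal reaches a small threshold.
; SelectionBoxDrawEnd stops drawing and returns the last query result, which is not cleared when a new drag starts.
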(event EventBeginPlay)

(event Collision|EventActorBeginOverlap
  (params (OtherActor :type Actor%20Object%20Reference)))

(event EventSelectionBoxDrawStart
  (params (X :type Float%20%28single-precision%29) (Y :type Float%20%28single-precision%29))
  (bind _output_get (Variables|Default|SetSelectionBoxStartX X))
  (bind _output_get_2 (Variables|Default|SetSelectionBoxStartY Y))
  (Variables|Default|SetSelectionBoxCurrentX _output_get)
  (Variables|Default|SetSelectionBoxCurrentY _output_get_2)
  (Variables|Default|SetisDrawingSelectionBox true))

(event EventTick
  (params (DeltaSeconds :type Float%20%28single-precision%29)))

(event EventSelectionBoxDrawUpdate
  (params (X :type Float%20%28single-precision%29) (Y :type Float%20%28single-precision%29))
  (Variables|Default|SetSelectionBoxCurrentX X)
  (Variables|Default|SetSelectionBoxCurrentY Y))

(event EventDrawHUD
  (params (SizeX :type Integer) (SizeY :type Integer))
  (bind _selectionboxcurrentx (Variables|Default|GetSelectionBoxCurrentX))
  (bind _selectionboxstarty (Variables|Default|GetSelectionBoxStartY))
  (bind _selectionboxstartx (Variables|Default|GetSelectionBoxStartX))
  (bind _selectionboxcurrenty (Variables|Default|GetSelectionBoxCurrentY))
  (if (Variables|Default|GetisDrawingSelectionBox)
    (if (>= (Math|Vector2D|Vector2DLength (- (Math|Vector2D|MakeVector2D (Variables|Default|GetSelectionBoxStartX) (Variables|Default|GetSelectionBoxStartY)) (Math|Vector2D|MakeVector2D (Variables|Default|GetSelectionBoxCurrentX) (Variables|Default|GetSelectionBoxCurrentY)))) 2e+01)
      (Utilities|FlowControl|Sequence
        (:then_0
          (Class|HUD|DrawLine (Variables|Default|GetSelectionBoxStartX) _selectionboxstarty (Variables|Default|GetSelectionBoxCurrentX) _selectionboxstarty "(R=0,G=0,B=0,A=1)" 5.0)
          (Class|HUD|DrawLine _selectionboxstartx (Variables|Default|GetSelectionBoxStartY) _selectionboxstartx (Variables|Default|GetSelectionBoxCurrentY) "(R=0,G=0,B=0,A=1)" 5.0)
          (Class|HUD|DrawLine (Variables|Default|GetSelectionBoxCurrentX) _selectionboxcurrenty (Variables|Default|GetSelectionBoxStartX) _selectionboxcurrenty "(R=0,G=0,B=0,A=1)" 5.0)
          (Class|HUD|DrawLine _selectionboxcurrentx (Variables|Default|GetSelectionBoxCurrentY) _selectionboxcurrentx (Variables|Default|GetSelectionBoxStartY) "(R=0,G=0,B=0,A=1)" 5.0)
          (Variables|Default|SetFoundActors (Class|HUD|GetActorsinSelectionRectangle "/Game/Blueprints/Vehicles/Abstract/BaseVehicle.BaseVehicle_C" (Math|Vector2D|MakeVector2D (Variables|Default|GetSelectionBoxStartX) (Variables|Default|GetSelectionBoxStartY)) (Math|Vector2D|MakeVector2D (Variables|Default|GetSelectionBoxCurrentX) (Variables|Default|GetSelectionBoxCurrentY)) false false)))))))

(fn ConstructionScript)

(fn SelectionBoxDrawEnd
  (Variables|Default|SetisDrawingSelectionBox false)
  (return (Variables|Default|GetFoundActors)))