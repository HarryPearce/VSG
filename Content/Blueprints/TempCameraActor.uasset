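; RTS-style control pawn that handles mouse selection, hovering and orders for units.
; A short timer separates double-clicks, which possess the controllable vehicle under the cursor, from clicks or drags.
; Drags select actors through a HUD-drawn box, while short clicks trace under the cursor, both using BPI_Selectable.
; Alt-fire traces from the mouse and orders selected units to attack BPI_Damagable hits or move to the hit location.
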(event Custom|LMB%20Pressed
  (Class|BPIRTSHud|SelectionBoxDrawStart(Message) (Variables|Default|GetHud) (Variables|Default|GetSelectionStartX) (Variables|Default|GetSelectionStartY))
  (Variables|Default|SetIsDrawing true))

(event Custom|LMB%20Released
  (bind _returnvalue (Game|GetPlayerController 0))
  (bind _pc (Variables|Default|GetPC))
  (bind _currentlyselectedactors (Variables|Default|GetCurrentlySelectedActors))
  (bind (_hitresult _returnvalue_2) (Game|Player|GetHitResultUnderCursorbyChannel _returnvalue "TraceTypeQuery4" true))
  (bind (_locationx _locationy) (Game|Player|GetMousePosition _pc))
  (bind _hitactor (Collision|BreakHitResult _hitresult))
  (Variables|Default|SetIsDrawing false)
  (bind _selectedactors (Class|BPIRTSHud|SelectionBoxDrawEnd(Message) (Variables|Default|GetHud)))
  (Utilities|FlowControl|Sequence
    (:then_0
      (Utilities|UnselectCurrentActors
        (:Completed
          (if (< 2e+01 (Math|Float|Absolute(Float) (Math|Vector2D|Vector2DLength (- (Math|Vector2D|MakeVector2D (Variables|Default|GetSelectionStartX) (Variables|Default|GetSelectionStartY)) (Math|Vector2D|MakeVector2D _locationx _locationy)))))
            (|SetCurrentlySelectedActors _selectedactors)
            (elif _returnvalue_2
              (bind _asbpi_selectable (Utilities|Casting|CastToBPI_Selectable _hitactor))
              (Development|PrintString (Utilities|GetDisplayName _hitactor))
              (Class|BPISelectable|Select(Message) _hitactor)
              (Utilities|Array|Clear _currentlyselectedactors)
              (Utilities|Array|Add _currentlyselectedactors _asbpi_selectable))))))
    (:then_1
      (Variables|Default|SetSelectionStartX 0.0)
      (Variables|Default|SetSelectionStartY 0.0)
      (Variables|Default|SetSelectionDrawTime 0.0))))

(event Custom|CheckIfIsPressed
  (Utilities|Time|ClearandInvalidateTimerbyHandle (Variables|Default|GetDoubleClickTimer))
  (CallFunction|LMBPressed)
  (if (not (Game|Player|IsInputKeyDown (Game|GetPlayerController 0) "LeftMouseButton"))
    (Utilities|FlowControl|DoOnce true) ; enters at Reset
  ))

(event Custom|DoubleClick
  (Pawn|Possess))

(event Collision|EventActorBeginOverlap
  (params (OtherActor :type Actor%20Object%20Reference)))

(event EventPossessed
  (params (NewController :type Controller%20Object%20Reference))
  (bind _asplayer_controller (Utilities|Casting|CastToPlayerController NewController))
  (bind _output_get (Variables|Default|SetPC _asplayer_controller))
  (Variables|Default|SetHud (HUD|GetHUD _output_get))
  (Variables|/Script/Engine.PlayerController|SetbShowMouseCursor (Variables|Default|GetPC) true))

(event EventFire
  (params (Pressed :type Boolean))
  (bind _pc (Variables|Default|GetPC))
  (bind (_locationx _locationy) (Game|Player|GetMousePosition _pc))
  (if Pressed
    (if (Utilities|Time|IsTimerActivebyHandle (Variables|Default|GetDoubleClickTimer))
      (Variables|Default|SetisDoubleClick true)
      (Utilities|Time|ClearandInvalidateTimerbyHandle (Variables|Default|GetDoubleClickTimer))
      (CallFunction|DoubleClick)
      (else
        (Variables|Default|SetSelectionStartX _locationx)
        (Variables|Default|SetSelectionStartY _locationy)
        (bind _returnvalue (Utilities|Time|SetTimerbyEvent (delegate Custom|CheckIfIsPressed) 0.15))
        (Variables|Default|SetDoubleClickTimer _returnvalue)))
    (elif (not (Utilities|Time|IsTimerActivebyHandle (Variables|Default|GetDoubleClickTimer)))
      (if (Variables|Default|GetisDoubleClick)
        (Variables|Default|SetisDoubleClick false)
        (else
          (CallFunction|LMBReleased))))))

(event EventTick
  (params (DeltaSeconds :type Float%20%28single-precision%29))
  (bind _pc (Variables|Default|GetPC))
  (bind (_locationx _locationy) (Game|Player|GetMousePosition _pc))
  (Utilities|FlowControl|Sequence
    (:then_0
      (Utilities|FlowControl|DoOnce true :!label _label
        (:Completed
          (CallFunction|LMBReleased))))
    (:then_1
      (if (Variables|Default|GetIsDrawing)
        (Variables|Default|SetSelectionDrawTime (+ DeltaSeconds (Variables|Default|GetSelectionDrawTime)))
        (Class|BPIRTSHud|SelectionBoxDrawUpdate(Message) (Variables|Default|GetHud) _locationx _locationy)
        (Utilities|FlowControl|DoOnce true
          (:Completed
            (goto _label Reset)))
        (else
          (|Hovering))))))

(event EventAltFire
  (params (Pressed :type Boolean))
  (bind _pc (Variables|Default|GetPC))
  (bind (_locationx _locationy) (Game|Player|GetMousePosition _pc))
  (bind (_worldposition _worlddirection) (Class|GameplayStatics|DeprojectScreentoWorld _pc (Math|Vector2D|MakeVector2D _locationx _locationy)))
  (if Pressed
    (for _array_element (Variables|Default|GetCurrentlySelectedActors)
      (bind (_outhit _returnvalue) (Collision|LineTraceByChannel _worldposition (+ _worldposition (* _worlddirection 2e+04)) "TraceTypeQuery1" false 0 "None"))
      (if _returnvalue
        (if (Utilities|DoesObjectImplementInterface (.HitActor (Collision|BreakHitResult _outhit)) "/Game/Blueprints/Interfaces/BPI_Damagable.BPI_Damagable_C")
          (Default|Attack _array_element (.HitActor (Collision|BreakHitResult _outhit)))
          (else
            (Default|Move _array_element (.Location (Collision|BreakHitResult _outhit)))))))))

(fn ConstructionScript)