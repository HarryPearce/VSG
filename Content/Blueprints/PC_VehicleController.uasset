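; Player controller for drivable vehicles that relays driving, flight, look, weapon and camera inputs to the possessed pawn as interface messages.
; Macros check that the pawn implements BPI_VehicleController_Controllable; the action macro derives KeyPressed from a FlipFlop shared by press and release.
; Camera switch, hover and alt-fire forward only when KeyPressed is true.
; PossessVehicle possesses a given vehicle and calls its OnPossess.
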(event EventBeginPlay
  (bind _controlledpawn (Utilities|IsPawnControllableAxis)
    (:True
      (Development|PrintString (Utilities|GetDisplayName _controlledpawn)))))

(event EventPossessVehicle
  (params (Vehicle :type BPI%20Vehicle%20Controller%20Controllable%20Interface))
  (bind _aspawn (Utilities|Casting|CastToPawn Vehicle))
  (Pawn|Possess _aspawn)
  (Default|OnPossess Vehicle))

(event Input|ActionEvents|InputActionStop
  (params (Key :type Key%20Structure :default "AnyKey"))
  ;[1 1 1] Action Input
  (:Pressed
    (bind (_controlledpawn _keypressed) (Utilities|IsPawnControllableAction :!label _label)
      (:True
        (Class|BPIVehicleControllerControllable|Stop(Message) _controlledpawn _keypressed))))
  (:Released
    (goto _label Released)))

(event Input|ActionEvents|InputActionFire
  (params (Key :type Key%20Structure :default "AnyKey"))
  ;[1 1 1] Action Input
  (:Pressed
    (bind (_controlledpawn _keypressed) (Utilities|IsPawnControllableAction :!label _label)
      (:True
        (Class|BPIVehicleControllerControllable|Fire(Message) _controlledpawn _keypressed))))
  (:Released
    (goto _label Released)))

(event Input|ActionEvents|InputActionSwitchCamera
  (params (Key :type Key%20Structure :default "AnyKey"))
  ;[1 1 1] Action Input
  (:Pressed
    (bind (_controlledpawn _keypressed) (Utilities|IsPawnControllableAction :!label _label)
      (:True
        (if _keypressed
          (Class|BPIVehicleControllerControllable|SwitchCamera(Message) _controlledpawn)))))
  (:Released
    (goto _label Released)))

(event Input|ActionEvents|InputActionHandbrake
  (params (Key :type Key%20Structure :default "AnyKey"))
  ;[1 1 1] Action Input
  (:Pressed
    (bind (_controlledpawn _keypressed) (Utilities|IsPawnControllableAction :!label _label)
      (:True
        (Class|BPIVehicleControllerControllable|Brake(Message) _controlledpawn _keypressed))))
  (:Released
    (goto _label Released)))

(event Input|ActionEvents|InputActionSetHover
  (params (Key :type Key%20Structure :default "AnyKey"))
  ;[1 1 1] Action Input
  (:Pressed
    (bind (_controlledpawn _keypressed) (Utilities|IsPawnControllableAction :!label _label)
      (:True
        (if _keypressed
          (Class|BPIVehicleControllerControllable|SetHover(Message) _controlledpawn _keypressed)))))
  (:Released
    (goto _label Released)))

(event Input|ActionEvents|InputActionAltFire
  (params (Key :type Key%20Structure :default "AnyKey"))
  ;[1 1 1] Action Input
  (:Pressed
    (bind (_controlledpawn _keypressed) (Utilities|IsPawnControllableAction :!label _label)
      (:True
        _)
      (:False
        _))
    (if _keypressed
      (Class|BPIVehicleControllerControllable|AltFire(Message) _controlledpawn _keypressed)))
  (:Released
    (goto _label Released)))

(event Input|AxisEvents|InputAxisLookUp
  (params (AxisValue :type Float%20%28single-precision%29))
  ;[1 1 1] Axis Input
  (bind _controlledpawn (Utilities|IsPawnControllableAxis)
    (:True
      (Class|BPIVehicleControllerControllable|LookUp(Message) _controlledpawn AxisValue))))

(event Input|AxisEvents|InputAxisMoveRight
  (params (AxisValue :type Float%20%28single-precision%29))
  ;[1 1 1] Axis Input
  (bind _controlledpawn (Utilities|IsPawnControllableAxis)
    (:True
      (Class|BPIVehicleControllerControllable|MoveRight(Message) _controlledpawn AxisValue))))

(event Input|AxisEvents|InputAxisMoveUP
  (params (AxisValue :type Float%20%28single-precision%29))
  ;[1 1 1] Axis Input
  (bind _controlledpawn (Utilities|IsPawnControllableAxis)
    (:True
      (Class|BPIVehicleControllerControllable|MoveUp(Message) _controlledpawn AxisValue))))

(event Input|AxisEvents|InputAxisMoveForward
  (params (AxisValue :type Float%20%28single-precision%29))
  ;[1 1 1] Axis Input
  (bind _controlledpawn (Utilities|IsPawnControllableAxis)
    (:True
      (Class|BPIVehicleControllerControllable|MoveForward(Message) _controlledpawn AxisValue))))

(event Input|AxisEvents|InputAxisLookRight
  (params (AxisValue :type Float%20%28single-precision%29))
  ;[1 1 1] Axis Input
  (bind _controlledpawn (Utilities|IsPawnControllableAxis)
    (:True
      (Class|BPIVehicleControllerControllable|LookRight(Message) _controlledpawn AxisValue))))

(fn ConstructionScript)