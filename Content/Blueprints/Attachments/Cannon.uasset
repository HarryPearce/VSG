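; Cannon attachment Blueprint that detects damageable actors in its line of fire.
; Each tick, after the parent logic, it runs a debug-drawn Visibility line trace forward from the projectile spawn component.
; A hit actor implementing BPI_Damagable becomes Target, which this graph never clears.
; The file contains no firing logic, and the construction script only calls the parent.
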(event EventTick
  (params (DeltaSeconds :type Float%20%28single-precision%29))
  (bind _projectilespawnclass (Variables|Default|GetProjectileSpawnClass))
  (bind _returnvalue (Transformation|GetWorldLocation _projectilespawnclass))
  (|CallParentFunction DeltaSeconds)
  (bind (_outhit _returnvalue_2) (Collision|LineTraceByChannel _returnvalue (+ _returnvalue (* (Math|Vector|GetForwardVector _projectilespawnclass) 5e+03)) "TraceTypeQuery1" false 0 "ForOneFrame"))
  (if _returnvalue_2
    (if (Utilities|DoesObjectImplementInterface (.HitActor (Collision|BreakHitResult _outhit)) "/Game/Blueprints/Interfaces/BPI_Damagable.BPI_Damagable_C")
      (Variables|Default|SetTarget (.HitActor (Collision|BreakHitResult _outhit))))))

(fn ConstructionScript
  (|CallParentFunction))