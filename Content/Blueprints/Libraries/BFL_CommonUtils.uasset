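; Blueprint function library of shared helpers for the modular vehicle attachment system, plus general array and path utilities.
; Socket helpers search by partial display name, compare actor extents against optional socket bounds, and resolve the owning BaseVehicle through AttachedTo links.
; Other helpers merge unique items, intersect arrays, subtract from float arrays, find the nearest point in an array or nav path, and pick the main attachment by socket type.
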(fn GetSocketbyDisplayName
  (params (Name :type String) (Sockets :type Array%20of%20Attachment%20Socket%20Object%20References))
  (bind _array_element (Utilities|Array|ForEachLoopwithBreak Sockets :!label _label)
    (:LoopBody
      (if (Utilities|String|Contains (Utilities|GetDisplayName _array_element) Name)
        (LocalVariables|SetRet _array_element)
        (goto _label Break)))
    (:Completed
      (return (LocalVariables|GetRet) (Utilities|IsValid (LocalVariables|GetRet))))))

(fn GetSocketbyDisplayNameGeneric
  (params (Name :type String) (Sockets :type Array%20of%20Scene%20Component%20Object%20References))
  (bind _array_element (Utilities|Array|ForEachLoopwithBreak Sockets :!label _label)
    (:LoopBody
      (if (Utilities|String|Contains (Utilities|GetDisplayName _array_element) Name)
        (LocalVariables|SetRet _array_element)
        (goto _label Break)))
    (:Completed
      (bind _asattachment_socket (Utilities|Casting|CastToAttachmentSocket (LocalVariables|GetRet))
        (:then
          (return _asattachment_socket false))
        (:CastFailed
          (return 0 true))))))

(fn IsActorinSocketBounds
  (params (Actor :type Actor%20Object%20Reference) (Socket :type Attachment%20Socket%20Object%20Reference))
  (bind (_origin _boxextent) (Collision|GetActorBounds Actor true))
  (bind _boundorigin (Variables|/Game/Blueprints/Sockets/AttachmentSocket.AttachmentSocket_C|GetBoundOrigin Socket))
  (bind _boundextent (Variables|/Game/Blueprints/Sockets/AttachmentSocket.AttachmentSocket_C|GetBoundExtent Socket))
  (bind _returnvalue (- _origin _boundorigin))
  (bind _returnvalue_2 (- _returnvalue _boxextent))
  (bind _returnvalue_3 (- _returnvalue _boundextent))
  (bind _returnvalue_4 (+ _boundextent _returnvalue))
  (bind _returnvalue_5 (+ _boxextent _returnvalue))
  (return (or (not (Variables|/Game/Blueprints/Sockets/AttachmentSocket.AttachmentSocket_C|GetHasBounds Socket)) (and (Math|Boolean|ANDBoolean (> (.x _returnvalue_5) (.x _returnvalue_4)) (> (.y _returnvalue_5) (.y _returnvalue_4)) (> (.z _returnvalue_5) (.z _returnvalue_4))) (Math|Boolean|ANDBoolean (< (.x _returnvalue_2) (.x _returnvalue_3)) (< (.y _returnvalue_2) (.y _returnvalue_3)) (< (.z _returnvalue_2) (.z _returnvalue_3)))))))

(fn GetSocketBaseVehicle
  (params (Socket :type Attachment%20Socket%20Object%20Reference))
  (bind _output_get (LocalVariables|SetActor (Components|GetOwner Socket)))
  (bind _asbase_vehicle (Utilities|Casting|CastToBaseVehicle _output_get)
    (:then
      (return _asbase_vehicle (LocalVariables|GetSuc)))
    (:CastFailed
      (while (LocalVariables|GetFoundBaseVehicle)
        (bind _asbase_attachment (Utilities|Casting|CastToBaseAttachment (LocalVariables|GetActor))
          (:then
            (bind _output_get_2 (LocalVariables|SetActor (Components|GetOwner (Variables|/Game/Blueprints/Attachments/Abstract/BaseAttachment.BaseAttachment_C|GetAttachedTo _asbase_attachment))))
            (Utilities|IsValid _output_get_2
              (:Is%20Valid
                (bind _asbase_vehicle_2 (Utilities|Casting|CastToBaseVehicle _output_get_2))
                (LocalVariables|SetBV _asbase_vehicle_2)
                (LocalVariables|SetFoundBaseVehicle false))
              (:Is%20Not%20Valid
                (LocalVariables|SetFoundBaseVehicle false)
                (LocalVariables|SetSuc false))))
          (:CastFailed
            (LocalVariables|SetFoundBaseVehicle false)
            (LocalVariables|SetSuc false))))
      (return (LocalVariables|GetBV) (LocalVariables|GetSuc)))))

(fn ArrayAddRange
  (params (A :type Array%20of%20Object%20Object%20References) (B :type Array%20of%20Object%20Object%20References))
  (for _array_element B
    (if (not (Utilities|Array|ContainsItem A _array_element))
      (Utilities|Array|Add A _array_element)))
  (return A))

(fn ArrayIntersect
  (params (A :type Array%20of%20Object%20Object%20References) (B :type Array%20of%20Object%20Object%20References))
  (for _array_element A
    (if (Utilities|Array|ContainsItem B _array_element)
      (Utilities|Array|Add (LocalVariables|GetOut) _array_element)))
  (return (LocalVariables|GetOut)))

(fn SubtractFloatfromArray
  (params (Array :type Array%20of%20Floats%20%28single-precision%29) (Num :type Float%20%28single-precision%29))
  (for (_array_element _array_index) Array
    (Utilities|Array|SetArrayElem Array _array_index (- _array_element Num)))
  (return Array))

(fn GetPointClosesttoinArray
  (params (Point :type Vector%20%28by%20ref%29) (Array :type Array%20of%20Vectors))
  (for (_array_element _array_index) Array
    (if (or (< (LocalVariables|GetClosestDistance) 0.0) (> (LocalVariables|GetClosestDistance) (Math|Vector|VectorLength (- Point _array_element))))
      (LocalVariables|SetClosestDistance (Math|Vector|VectorLength (- Point _array_element)))
      (LocalVariables|SetClosesetIndex _array_index)))
  (return (Utilities|Array|Get(acopy) Array (LocalVariables|GetClosesetIndex)) (LocalVariables|GetClosesetIndex)))

(fn GetPointClosesttoinPath
  (params (Point :type Vector%20%28by%20ref%29) (NavPath :type Navigation%20Path%20Object%20Reference%20%28by%20ref%29))
  (bind _pathpoints (Variables|/Script/Engine.NavigationPath|GetPathPoints NavPath))
  (for (_array_element _array_index) _pathpoints
    (if (or (< (LocalVariables|GetClosestDistance) 0.0) (> (LocalVariables|GetClosestDistance) (Math|Vector|VectorLength (- Point _array_element))))
      (LocalVariables|SetClosestDistance (Math|Vector|VectorLength (- Point _array_element)))
      (LocalVariables|SetClosesetIndex _array_index)))
  (return (Utilities|Array|Get(acopy) _pathpoints (LocalVariables|GetClosesetIndex)) (LocalVariables|GetClosesetIndex)))

(fn GetMainAttachmentfromArray
  (params (ControllableAttachments :type Array%20of%20Controllable%20Attachment%20Object%20References))
  (for _array_element ControllableAttachments
    (if (Utilities|Enum|Equal(Enum) (Variables|/Game/Blueprints/Sockets/AttachmentSocket.AttachmentSocket_C|GetAttachmentType (Variables|/Game/Blueprints/Attachments/Abstract/BaseAttachment.BaseAttachment_C|GetAttachedTo _array_element)) "NewEnumerator0")
      (LocalVariables|SetRet _array_element)))
  (return (LocalVariables|GetRet)))