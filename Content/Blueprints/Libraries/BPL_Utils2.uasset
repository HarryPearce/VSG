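; Blueprint utility library with helpers for actor bounds, screen visibility and angles between direction vectors.
; GetActortBoundingBoxPoints builds the eight corners of an actor's bounds, and IsAnyPointVisible tests whether any given point projects inside player 0's viewport, without occlusion checks.
; PivotRotation returns horizontal and vertical radian offsets from Pivot to Rotation, using AcosAsinToRad to resolve full-circle angles and wrapping negative horizontal results.
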(fn GetActortBoundingBoxPoints
  (params (Actor :type Actor%20Object%20Reference) (OnlyCollidingComponents :type Boolean))
  (bind (_origin _boxextent) (Collision|GetActorBounds Actor OnlyCollidingComponents))
  (bind _returnvalue (* (.x _boxextent) -1.0))
  (bind _returnvalue_2 (* (.y _boxextent) -1.0))
  (bind _returnvalue_3 (* (.z _boxextent) -1.0))
  (bind _returnvalue_4 (+ (.x _origin) (.x _boxextent)))
  (bind _returnvalue_5 (+ (.y _origin) (.y _boxextent)))
  (bind _returnvalue_6 (+ (.z _origin) (.z _boxextent)))
  (bind _returnvalue_7 (+ (.x _origin) _returnvalue))
  (bind _returnvalue_8 (+ (.y _origin) _returnvalue_2))
  (bind _returnvalue_9 (+ (.z _origin) _returnvalue_3))
  (return (Utilities|Array|MakeArray (Math|Vector|MakeVector _returnvalue_4 _returnvalue_5 _returnvalue_6) (Math|Vector|MakeVector _returnvalue_7 _returnvalue_5 _returnvalue_6) (Math|Vector|MakeVector _returnvalue_4 _returnvalue_8 _returnvalue_6) (Math|Vector|MakeVector _returnvalue_4 _returnvalue_5 _returnvalue_9) (Math|Vector|MakeVector _returnvalue_4 _returnvalue_8 _returnvalue_9) (Math|Vector|MakeVector _returnvalue_7 _returnvalue_5 _returnvalue_9) (Math|Vector|MakeVector _returnvalue_7 _returnvalue_8 _returnvalue_6) (Math|Vector|MakeVector _returnvalue_7 _returnvalue_8 _returnvalue_9))))

(fn IsAnyPointVisible
  (params (Array :type Array%20of%20Vectors))
  (bind _returnvalue (Game|GetPlayerController 0))
  (bind (_sizex _sizey) (HUD|GetViewportSize _returnvalue))
  (for _array_element Array
    (if (Math|Boolean|ANDBoolean (>= (.x (.ScreenLocation (Class|PlayerController|ProjectWorldLocationtoScreen _returnvalue _array_element false))) 0.0) (>= (.y (.ScreenLocation (Class|PlayerController|ProjectWorldLocationtoScreen _returnvalue _array_element false))) 0.0) (<= (.x (.ScreenLocation (Class|PlayerController|ProjectWorldLocationtoScreen _returnvalue _array_element false))) (Math|Conversions|ToFloat(Integer) _sizex)) (<= (.y (.ScreenLocation (Class|PlayerController|ProjectWorldLocationtoScreen _returnvalue _array_element false))) (Math|Conversions|ToFloat(Integer) _sizey)))
      (LocalVariables|SetretVal true)))
  (return (LocalVariables|GetretVal)))

(fn AcosAsintoRad
  (params (Asin :type Float%20%28single-precision%29) (Acos :type Float%20%28single-precision%29))
  (return (select (< Asin 0.0) (- (* (Math|Trig|GetPI) 2.0) Acos) Acos)))

(fn PivotRotation
  (params (Pivot :type Vector) (Rotation :type Vector))
  (bind _returnvalue (Class|KismetMathLibrary|Asin (.x Rotation)))
  (bind _returnvalue_2 (Class|KismetMathLibrary|Asin (.x Pivot)))
  (bind _returnvalue_3 (Math|Trig|Acos(Degrees) (.y Pivot)))
  (bind _returnvalue_4 (Math|Trig|Acos(Degrees) (.y Rotation)))
  (bind _rad (CallFunction|AcosAsintoRad _returnvalue_2 _returnvalue_3))
  (bind _rad_2 (CallFunction|AcosAsintoRad _returnvalue _returnvalue_4))
  (bind _returnvalue_5 (- _rad_2 _rad))
  (return (select (< _returnvalue_5 0.0) (+ _returnvalue_5 (* (Math|Trig|GetPI) 2.0)) _returnvalue_5) (- (Math|Trig|Acos(Degrees) (.z Rotation)) (Math|Trig|Acos(Degrees) (.z Pivot)))))